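; Game mode for the Wind Razor that scripts mission progression from opening Skipper orders through scout plane, smokes errand and enemy plane waves.
; BeginPlay caches Kreige fighters, resumes from PlayerProgress and starts a looping kill check.
; Waves activate fighters by WaveID; reaching the kill quota ends raids, fades music and triggers follow-up by wave, guarded by a resettable DoOnce.
; It also tracks ship health; the repairs stage is an empty stub.
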(event Custom|DamageShip
  (params (Damage :type Integer))
  (bind _output_get (Variables|Default|SetWindRazorHealth (- (Variables|Default|GetWindRazorHealth) Damage)))
  (Development|PrintString (Utilities|String|ToString(Integer) _output_get) true true "(R=1.000000,G=0.750000,B=0.000000,A=1.000000)" 5.0))

(event Custom|TriggerGetSmokes
  ;[0.8027 1 0.6652] Retrieve Smokes
  (Variables|Default|SetPlayerProgress 2)
  (Default|HighlightObject (Variables|Default|GetSmokes)))

(event Custom|TriggerRepairs
  ;[1 0.06809 0] Put Out Those Fires
)

(event Custom|TriggerWave1
  ;[0.1071 1 0] Wave 1
  (CallFunction|ResetCounter)
  (Utilities|FlowControl|DoOnce false
    (:Completed
      (Variables|Default|SetCurrentWave 1)
      (Variables|Default|SetPlanesDestroyed 0)
      (Variables|Default|SetNumPlanesToDestroy 15)
      (Audio|PlaySound2D "/Game/Audio/VOX/SC_CoPilot_Line2.SC_CoPilot_Line2")
      (for _array_element (Variables|Default|GetEnemyPlanes)
        (if (== (Variables|/Game/Blueprints/Actors/BP_KreigeFighter.BP_KreigeFighter_C|GetWaveID _array_element) 1)
          (Default|WaveStart _array_element))))))

(event Custom|TriggerPlaneRush
  ;[1 0.934 0.1302] PlaneRush
  (Variables|Default|SetCurrentWave 8)
  (for _array_element (Variables|Default|GetEnemyPlanes)
    (if (== (Variables|/Game/Blueprints/Actors/BP_KreigeFighter.BP_KreigeFighter_C|GetWaveID _array_element) 8)
      (Default|WaveStart _array_element)
      (Utilities|FlowControl|Delay 2.0)
      (Default|IncomingEnemies (Variables|Default|GetSkipper))
      (CallFunction|PlayMusic))))

(event Custom|Play%20Music
  (Audio|Components|Audio|Play (Variables|Default|GetMusic) 0.0))

(event Custom|CheckPlanes
  (bind _planesdestroyed (Variables|Default|GetPlanesDestroyed))
  ;[1 0.934 0] Plane Counter
  (Development|PrintString (Utilities|String|ToString(Integer) _planesdestroyed))
  (if (>= _planesdestroyed (Variables|Default|GetNumPlanesToDestroy))
    (CallFunction|StopWave)))

(event Custom|Reset%20Counter
  ;[1 0 0] Stop Wave
  (Utilities|FlowControl|DoOnce false) ; enters at Reset
)

(event Custom|StopWave
  ;[1 0 0] Stop Wave
  (Utilities|FlowControl|DoOnce false
    (:Completed
      (for _array_element (Variables|Default|GetEnemyPlanes)
        (Default|EndRaid _array_element)
        (Audio|Components|Audio|FadeOut (Variables|Default|GetMusic) 5.0 0.0 :!class /Script/Engine.AudioComponent))
      (Utilities|FlowControl|Delay 4.0)
      (switch int (Variables|Default|GetCurrentWave)
        (:0
          (Default|VOSmokes (Variables|Default|GetSkipper)))
        (:1
          (CallFunction|TriggerRepairs))))))

(event Custom|TriggerScoutPlane
  ;[0 0.3168 1] Scout Plane
  (Variables|Default|SetPlayerProgress 1)
  (Utilities|FlowControl|DoOnce false
    (:Completed
      (Variables|Default|SetCurrentWave 0)
      (Variables|Default|SetPlanesDestroyed 0)
      (Variables|Default|SetNumPlanesToDestroy 1)
      (for _array_element (Variables|Default|GetEnemyPlanes)
        (if (== (Variables|/Game/Blueprints/Actors/BP_KreigeFighter.BP_KreigeFighter_C|GetWaveID _array_element) 0)
          (Default|WaveStart _array_element))))))

(event Custom|Ring%20Transmitter
  ;[1 1 1] Starting Orders
  (Default|TransmitterRing (Variables|Default|GetTransmitter))
  (Utilities|FlowControl|Delay 3.0)
  (Default|VORightO (Variables|Default|GetSkipper)))

(event Custom|TriggerFirstOrders
  ;[1 1 1] Starting Orders
  (Utilities|FlowControl|Delay 5.0)
  (Default|VORiseandShine (Variables|Default|GetSkipper)))

(event Custom|Orders%20Given
  ;[1 1 1] Starting Orders
  (Utilities|FlowControl|Delay 3.0)
  (Default|VOBugger (Variables|Default|GetSkipper)))

(event Custom|TriggerSmokesGiven
  ;[0.8027 1 0.6652] Retrieve Smokes
  (Variables|Default|SetPlayerProgress 3)
  (Utilities|FlowControl|Delay 3.0)
  (Default|IncomingTransmission (Variables|Default|GetSkipper)))

(event Custom|ShipDestroyed
  (Math|Integer|IncrementInt (Variables|Default|GetPlanesDestroyed)
    (:%20%20
      (CallFunction|CheckPlanes))))

(event EventBeginPlay
  (bind _outactors (Actor|GetAllActorsOfClass "/Game/Blueprints/Actors/BP_KreigeFighter.BP_KreigeFighter_C"))
  (Variables|Default|SetEnemyPlanes _outactors)
  (Utilities|Time|SetTimerbyFunctionName 0 "CheckPlanes" 1.0 true)
  (switch int (Variables|Default|GetPlayerProgress)
    (:Default
      (CallFunction|TriggerFirstOrders :!label _label))
    (:0
      (goto _label))
    (:1
      (CallFunction|TriggerScoutPlane))
    (:2
      (CallFunction|TriggerGetSmokes))
    (:3
      (CallFunction|TriggerSmokesGiven))))

(fn ConstructionScript)