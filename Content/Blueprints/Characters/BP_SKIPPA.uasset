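; BP_SKIPPA is the Skippa character, who voices scripted dialogue to Rook and advances the WindRazor mission sequence.
; Each event plays 2D dialogue or sound, waits out the clip's duration, and most then call a WindRazorGameMode trigger for the next beat, such as scout plane, waves or repairs.
; Overlapping the game mode's Smokes actor destroys it, shows the CapsCigs component and reports the smokes as given.
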(event Custom|VO_RiseAndShine
  ;[0.6094 0.2951 0.08925] Dialogue Players
  (Class|GameplayStatics|PlayDialogue2D (Variables|Default|GetRise'n'ShineSUB) (Variables|Default|GetToRook))
  (Utilities|FlowControl|Delay (Variables|/Script/Engine.SoundBase|GetDuration (Variables|Default|GetRise'n'Shine)))
  (Default|RingTransmitter (stale EventBeginPlay _aswind_razor_game_mode)))

(event Custom|Incoming%20Transmission
  ;[0.6094 0.2951 0.08925] Dialogue Players
  (Audio|PlaySound2D "/Game/Audio/VOX/S_KriegeTransmission.S_KriegeTransmission")
  (Utilities|FlowControl|Delay (Variables|/Script/Engine.SoundBase|GetDuration (Variables|Default|GetKriegeTransmission)))
  (Class|GameplayStatics|PlayDialogue2D (Variables|Default|GetInterestingSUB) (Variables|Default|GetToRook))
  (Utilities|FlowControl|Delay (Variables|/Script/Engine.SoundBase|GetDuration (Variables|Default|GetInteresting)))
  (Default|TriggerPlaneRush (stale EventBeginPlay _aswind_razor_game_mode)))

(event Custom|VO_Smokes
  ;[0.6094 0.2951 0.08925] Dialogue Players
  (Class|GameplayStatics|PlayDialogue2D (Variables|Default|GetSmokesSUB) (Variables|Default|GetToRook))
  (Utilities|FlowControl|Delay (Variables|/Script/Engine.SoundBase|GetDuration (Variables|Default|GetSmokes)))
  (Default|TriggerGetSmokes (stale EventBeginPlay _aswind_razor_game_mode)))

(event Custom|IncomingEnemies
  (bind _torook (Variables|Default|GetToRook))
  (bind _howmany (Variables|Default|GetHowMany))
  ;[0.6094 0.2951 0.08925] Dialogue Players
  (Audio|PlaySound2D _howmany)
  (Utilities|FlowControl|Delay (Variables|/Script/Engine.SoundBase|GetDuration _howmany))
  (Class|GameplayStatics|PlayDialogue2D (Variables|Default|GetInFrontOfYouSUB) _torook)
  (Utilities|FlowControl|Delay (+ (Variables|/Script/Engine.SoundBase|GetDuration (Variables|Default|GetInFrontOfYou)) 3.0))
  (Class|GameplayStatics|PlayDialogue2D (Variables|Default|GetManThatAftSUB) _torook)
  (Utilities|FlowControl|Delay (Variables|/Script/Engine.SoundBase|GetDuration (Variables|Default|GetManThatAft)))
  (Default|TriggerWave1 (stale EventBeginPlay _aswind_razor_game_mode)))

(event Custom|VO_Bugger
  ;[0.6094 0.2951 0.08925] Dialogue Players
  (Class|GameplayStatics|PlayDialogue2D (Variables|Default|GetBuggerSUB) (Variables|Default|GetToRook))
  (Utilities|FlowControl|Delay (Variables|/Script/Engine.SoundBase|GetDuration (Variables|Default|GetBugger)))
  (Default|TriggerScoutPlane (stale EventBeginPlay _aswind_razor_game_mode)))

(event Custom|PutThatFireOut
  ;[0.6094 0.2951 0.08925] Dialogue Players
  (Class|GameplayStatics|PlayDialogue2D (Variables|Default|GetPutFireOutSUB) (Variables|Default|GetToRook))
  (Utilities|FlowControl|Delay (Variables|/Script/Engine.SoundBase|GetDuration (Variables|Default|GetPutFireOut)))
  (Default|TriggerRepairs (stale EventBeginPlay _aswind_razor_game_mode)))

(event Custom|VO_RightO
  ;[0.6094 0.2951 0.08925] Dialogue Players
  (Class|GameplayStatics|PlayDialogue2D (Variables|Default|GetRightOSUB) (Variables|Default|GetToRook))
  (Utilities|FlowControl|Delay (Variables|/Script/Engine.SoundBase|GetDuration (Variables|Default|GetRightO))))

(event EventBeginPlay
  ;[0 0 0] Cast Setup
  (bind _aswind_razor_game_mode (Utilities|Casting|CastToWindRazorGameMode (Game|GetGameMode))))

(event Collision|EventActorBeginOverlap
  (params (OtherActor :type Actor%20Object%20Reference))
  ;[0.6094 0.2951 0.08925] Dialogue Players
  (if (== OtherActor (Variables|/Game/Blueprints/WindRazorGameMode.WindRazorGameMode_C|GetSmokes (stale EventBeginPlay _aswind_razor_game_mode)))
    (Development|PrintString "good")
    (Actor|DestroyActor OtherActor)
    (Rendering|SetVisibility (Variables|Default|GetCapsCigs) true false)
    (Default|TriggerSmokesGiven (stale EventBeginPlay _aswind_razor_game_mode))
    (else
      (Development|PrintString "bad"))))

(fn ConstructionScript)