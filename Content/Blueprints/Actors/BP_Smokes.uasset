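; BP_Smokes is a grabbable pack prop that can be highlighted, picked up and dropped.
; Highlighting uses custom depth on the Pack component and sets ActiveOrders, which nothing here clears.
; Pickup disables physics, attaches the root to the supplied component and hides the highlight; Drop restores physics, detaches and re-highlights if ActiveOrders is set.
; The left and right trigger functions are stubs returning false.
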(event Custom|HighlightObject
  (Rendering|SetRenderCustomDepth (Variables|Default|GetPack) true)
  (Variables|Default|SetActiveOrders true))

(event Custom|RemoveHighlights
  (Variables|Default|SetHighlightsRemoved true)
  (Rendering|SetRenderCustomDepth (Variables|Default|GetPack) false))

(event EventPickup
  (params (AttachTo :type Scene%20Component%20Object%20Reference) (Hand :type EControllerHand%20Enum :default "Left"))
  (Physics|SetSimulatePhysics (Variables|Default|GetPack) false)
  (Transformation|AttachComponentToComponent (VehicleSound|GetRootComponent) AttachTo "None" "KeepWorld" "KeepWorld" "KeepWorld" true)
  (Rendering|SetRenderCustomDepth (Variables|Default|GetPack) false))

(event EventDrop
  (bind _pack (Variables|Default|GetPack))
  (Physics|SetSimulatePhysics _pack true)
  (Transformation|DetachFromActor "KeepWorld" "KeepWorld" "KeepWorld")
  (if (Variables|Default|GetActiveOrders)
    (Rendering|SetRenderCustomDepth _pack true)))

(fn ConstructionScript)

(fn PullLeftTrigger
  (params (Interactor :type BP%20Motion%20Controller%20Object%20Reference))
  (return false))

(fn PullRightTrigger
  (params (Interactor :type BP%20Motion%20Controller%20Object%20Reference))
  (return false))

(fn ReleaseLeftTrigger
  (params (Interactor :type BP%20Motion%20Controller%20Object%20Reference))
  (return false))

(fn ReleaseRightTrigger
  (params (Interactor :type BP%20Motion%20Controller%20Object%20Reference))
  (return false))