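; BP_RushingEnemy is an enemy actor that makes a single long straight rush.
; After a short delay on BeginPlay, if WillMove is set, a MoveComponentTo sends its StaticMesh far along +X over a random duration.
; The Destroy event stops that move, while Explode and Hit are empty.
; Disconnected leftover logic holds a ping-pong plane timeline, explosion spawn and physics-based death.
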(event Custom|Explode)

(event Custom|Destroy
  (bind _staticmesh (Variables|Default|GetStaticMesh))
  (Components|MoveComponentTo _staticmesh (+ (Transformation|GetWorldLocation _staticmesh) "300000.000000,0.000000, 0") (Transformation|GetWorldRotation _staticmesh) false false (Math|Random|RandomFloatinRange 4.0 6.0) false) ; enters at Stop
)

(event EventBeginPlay
  (bind _staticmesh (Variables|Default|GetStaticMesh))
  (Utilities|FlowControl|Delay 5.0)
  (if (Variables|Default|GetWillMove)
    (Components|MoveComponentTo _staticmesh (+ (Transformation|GetWorldLocation _staticmesh) "300000.000000,0.000000, 0") (Transformation|GetWorldRotation _staticmesh) false false (Math|Random|RandomFloatinRange 4.0 6.0) false)))

(event EventTick
  (params (DeltaSeconds :type Float%20%28single-precision%29)))

(event Collision|EventHit
  (params (MyComp :type Primitive%20Component%20Object%20Reference) (Other :type Actor%20Object%20Reference) (OtherComp :type Primitive%20Component%20Object%20Reference) (bSelfMoved :type Boolean) (HitLocation :type Vector :default "0, 0, 0") (HitNormal :type Vector :default "0, 0, 0") (NormalImpulse :type Vector :default "0, 0, 0") (Hit :type Hit%20Result%20Structure%20%28by%20ref%29))
  ;[1 1 1] Destroyed on Hit
)

(fn ConstructionScript)