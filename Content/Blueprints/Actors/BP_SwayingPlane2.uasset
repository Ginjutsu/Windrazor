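; BP_SwayingPlane2 is a plane actor that sways around its starting position and is destroyed when hit.
; After a random start delay, a timeline offsets the static mesh from its initial location, and the PlayedOnce flag alternates reverse and forward playback to loop the motion.
; On Hit it activates an explosion particle, then destroys itself after a short delay.
; The Explode event is empty and the fire-explosion spawn is disconnected.
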(event Custom|Explode)

(event Collision|EventHit
  (params (MyComp :type Primitive%20Component%20Object%20Reference) (Other :type Actor%20Object%20Reference) (OtherComp :type Primitive%20Component%20Object%20Reference) (bSelfMoved :type Boolean) (HitLocation :type Vector :default "0, 0, 0") (HitNormal :type Vector :default "0, 0, 0") (NormalImpulse :type Vector :default "0, 0, 0") (Hit :type Hit%20Result%20Structure%20%28by%20ref%29))
  ;[1 1 1] Destroyed on Hit
  (Components|Activation|Activate (Variables|Default|GetP_Explosion) false)
  (Utilities|FlowControl|Delay 0.2)
  (Actor|DestroyActor))

(event EventBeginPlay
  ;[1 1 1] Planes Movement
  (Utilities|FlowControl|Delay (Math|Random|RandomFloatinRange 0.0 1e+01))
  (Variables|Default|SetInitLoc (Transformation|GetWorldLocation (Variables|Default|GetStaticMesh)))
  (bind _planeloc (Timeline|PlaneLoc Play)
    (:Update
      (Transformation|SetWorldLocation (Variables|Default|GetStaticMesh) (+ _planeloc (Variables|Default|GetInitLoc)) false false))
    (:Finished
      (Utilities|FlowControl|Delay 0.2)
      (if (Variables|Default|GetPlayedOnce)
        (Variables|Default|SetPlayedOnce false)
        (Timeline|PlaneLoc PlayFromStart)
        (else
          (Variables|Default|SetPlayedOnce true)
          (Timeline|PlaneLoc Reverse))))))

(fn ConstructionScript)