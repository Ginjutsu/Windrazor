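; Grabbable comm phone receiver with a cable that rings on a transmitter call and delivers the HC orders audio.
; Pickup stops the ring, disables physics on the phone mesh and attaches it to the grabbing component; Drop restores physics and calls DetachFromActor.
; A game mode flag makes the orders play only on first pickup, and audio completion calls OrdersGiven on the game mode.
; Trigger interaction functions are stubs returning false.
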(event OnAudioFinished(HCOrders)
  (Default|OrdersGiven (stale EventPickup _aswind_razor_game_mode)))

(event Custom|TransmitterRing
  (Audio|Components|Audio|Play (Variables|Default|GetRing) 0.0))

(event EventPickup
  (params (AttachTo :type Scene%20Component%20Object%20Reference) (Hand :type EControllerHand%20Enum :default "Left"))
  (Audio|Components|Audio|Stop (Variables|Default|GetRing))
  (if (Variables|Default|GetIsInBase)
    (Development|PrintString "Phone CLICK ON"))
  (Physics|SetSimulatePhysics (Variables|Default|GetPhone) false)
  (Transformation|AttachComponentToComponent (Variables|Default|GetPhone) AttachTo "None" "KeepRelative" "KeepRelative" "KeepRelative" true)
  (bind _aswind_razor_game_mode (Utilities|Casting|CastToWindRazorGameMode (Game|GetGameMode)))
  (if (not (Variables|/Game/Blueprints/WindRazorGameMode.WindRazorGameMode_C|GetHCOrdersGiven _aswind_razor_game_mode))
    (Variables|/Game/Blueprints/WindRazorGameMode.WindRazorGameMode_C|SetHCOrdersGiven _aswind_razor_game_mode true)
    (Audio|Components|Audio|Play (Variables|Default|GetHCOrders) 0.0)))

(event EventDrop
  (Physics|SetSimulatePhysics (Variables|Default|GetPhone) true)
  (Transformation|DetachFromActor "KeepRelative" "KeepRelative" "KeepRelative"))

(fn ConstructionScript
  (Class|CableComponent|SetAttachEndto (Variables|Default|GetCable) 0 "None" "None"))

(fn PullLeftTrigger
  (params (Interactor :type BP%20Motion%20Controller%20Object%20Reference))
  (return false))

(fn PullRightTrigger
  (params (Interactor :type BP%20Motion%20Controller%20Object%20Reference))
  (return false))

(fn ReleaseLeftTrigger
  (params (Interactor :type BP%20Motion%20Controller%20Object%20Reference))
  (return false))

(fn ReleaseRightTrigger
  (params (Interactor :type BP%20Motion%20Controller%20Object%20Reference))
  (return false))