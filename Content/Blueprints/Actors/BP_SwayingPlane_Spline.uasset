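; BP_SwayingPlane_Spline is an enemy plane that flies along a spline and damages the player ship through WindRazorGameMode.
; WaveStart triggers a reset and randomly delayed respawn; Tick then advances the mesh by a fixed per-frame step, firing once past FiringDistance.
; Reaching the spline end or being hit, which plays explosion particles and hides the mesh, restarts the cycle.
; The construction script places a firing-point marker; older movement logic is left unconnected.
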(event Custom|Explode)

(event Custom|WaveStart
  (CallFunction|Reset))

(event Custom|reset
  (Rendering|Material|SetMaterial (Variables|Default|GetStaticMesh) 0 "/Game/Materials/EnemyPlane_Material.EnemyPlane_Material")
  (Variables|Default|Setflying false)
  (Variables|Default|SetdistanceFlown 0.0)
  (Utilities|FlowControl|Delay (Math|Random|RandomFloatinRange 5.0 1e+01))
  (Utilities|FlowControl|Sequence
    (:then_0
      (Utilities|FlowControl|DoOnce false) ; enters at Reset
    )
    (:then_1
      (CallFunction|Respawn))))

(event Custom|respawn
  (Variables|Default|SetPlaneDestroyed false)
  (Rendering|SetVisibility (Variables|Default|GetStaticMesh) true false)
  (Variables|Default|Setflying true))

(event Custom|Destroy
  (bind _staticmesh (Variables|Default|GetStaticMesh))
  (Components|MoveComponentTo _staticmesh (+ (Transformation|GetWorldLocation _staticmesh) "-80000.000000,0.000000, 0") (Transformation|GetWorldRotation _staticmesh) false false (Math|Random|RandomFloatinRange 18.0 25.0) false) ; enters at Stop
  (if (not (Variables|Default|GetPlaneDestroyed))
    (Actor|DestroyActor)))

(event Custom|Shoot
  (Rendering|Material|SetMaterial (Variables|Default|GetStaticMesh) 0 "/Game/Geometry/Blockout/Seth/lambert1.lambert1")
  (Default|DamageShip (Variables|Default|GetWindRazorGameMode) 2))

(event EventBeginPlay
  (bind _aswind_razor_game_mode (Utilities|Casting|CastToWindRazorGameMode (Game|GetGameMode)))
  (Variables|Default|SetWindRazorGameMode _aswind_razor_game_mode)
  (Utilities|FlowControl|Delay (Variables|Default|GetFlightDelay))
  (if (Variables|Default|GetWillMove)
    _))

(event EventTick
  (params (DeltaSeconds :type Float%20%28single-precision%29))
  (if (Variables|Default|Getflying)
    (if (Variables|Default|GetPlaneDestroyed)
      (CallFunction|Reset)
      (else
        (bind _output_get (Variables|Default|SetdistanceFlown (+ (Variables|Default|GetdistanceFlown) (Variables|Default|GetPlaneBaseSpeed))))
        (Transformation|SetWorldTransform (Variables|Default|GetStaticMesh) (Math|Transform|MakeTransform (.location (Spline|GetTransformatDistanceAlongSpline (Variables|Default|GetSpline) _output_get "World" false)) (Math|Rotator|MakeRotator (.roll (.rotation (Spline|GetTransformatDistanceAlongSpline (Variables|Default|GetSpline) _output_get "World" false))) (.pitch (.rotation (Spline|GetTransformatDistanceAlongSpline (Variables|Default|GetSpline) _output_get "World" false))) (.yaw (.rotation (Spline|GetTransformatDistanceAlongSpline (Variables|Default|GetSpline) _output_get "World" false)))) "2.000000,2.000000,2.000000") false false)
        (if (>= (Variables|Default|GetdistanceFlown) (Spline|GetSplineLength (Variables|Default|GetSpline)))
          (CallFunction|Reset)
          (elif (>= (Variables|Default|GetdistanceFlown) (Variables|Default|GetFiringDistance))
            (Utilities|FlowControl|DoOnce false
              (:Completed
                (CallFunction|Shoot)))))))))

(event Collision|EventHit
  (params (MyComp :type Primitive%20Component%20Object%20Reference) (Other :type Actor%20Object%20Reference) (OtherComp :type Primitive%20Component%20Object%20Reference) (bSelfMoved :type Boolean) (HitLocation :type Vector :default "0, 0, 0") (HitNormal :type Vector :default "0, 0, 0") (NormalImpulse :type Vector :default "0, 0, 0") (Hit :type Hit%20Result%20Structure%20%28by%20ref%29))
  ;[1 1 1] Destroyed on Hit
  (Utilities|FlowControl|DoOnce false :!label _label
    (:Completed
      (Components|Activation|Activate (Variables|Default|GetP_Explosion) false)
      (Rendering|SetVisibility (Variables|Default|GetStaticMesh) false false)
      (Variables|Default|SetPlaneDestroyed true)
      (Utilities|FlowControl|Delay 2.0)
      (goto _label Reset))))

(fn ConstructionScript
  (Transformation|SetWorldLocation (Variables|Default|GetFiringDistanceVisual) (Spline|GetLocationatDistanceAlongSpline (Variables|Default|GetSpline) (Variables|Default|GetFiringDistance) "World") false false))