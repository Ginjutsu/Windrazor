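; BP_SwayingPlane is an actor that makes its Bomber component drift and sway around its starting pose.
; On BeginPlay it stores the component's relative location and rotation.
; It then loops endlessly, easing to a random nearby offset with slight random pitch, then easing back more slowly to the stored pose, using latent MoveComponentTo calls with random durations.
; A zero Delay restarts each cycle.
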(event EventBeginPlay
  (bind _bomber (Variables|Default|GetBomber))
  (bind _bomber_2 (Variables|Default|GetBomber))
  (Variables|Default|SetInitLoc (Variables|/Script/Engine.SceneComponent|GetRelativeLocation _bomber))
  (Variables|Default|SetInitRot (Variables|/Script/Engine.SceneComponent|GetRelativeRotation _bomber))
  (Components|MoveComponentTo _bomber_2 (+ (Math|Vector|MakeVector (Math|Random|RandomFloatinRange -2e+03 2e+03) (Math|Random|RandomFloatinRange -1.5e+03 1.5e+03) (Math|Random|RandomFloatinRange -7e+02 7e+02)) (Variables|Default|GetInitLoc)) (Math|Rotator|CombineRotators (Math|Rotator|MakeRotator 0.0 (Math|Random|RandomFloatinRange -1e+01 1e+01) 0.0) (Variables|Default|GetInitRot)) true true (Math|Random|RandomFloatinRange 3.0 7.0) false :!label _label)
  (Components|MoveComponentTo _bomber_2 (Variables|Default|GetInitLoc) (Variables|Default|GetInitRot) true true (Math|Random|RandomFloatinRange 7.0 11.0) false)
  (Utilities|FlowControl|Delay 0.0)
  (goto _label))

(fn ConstructionScript)