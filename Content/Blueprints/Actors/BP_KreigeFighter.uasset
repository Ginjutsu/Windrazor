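; Enemy fighter plane that flies raid runs along a spline, respawning after a delay until the raid ends or its one-time flight completes.
; Tick advances it by distance; past FiringStartDistance, previewed by the construction script, it fires once per run.
; Firing is muzzle flashes plus delayed game-mode ship damage, skipped if the plane is downed first.
; BP_ElectroBullet hits deplete health, triggering a physics fall, explosion, game-mode notification and reset.
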(event Custom|DestroyPlane
  ;[0 0 0] Destroy Plane
  (Utilities|FlowControl|DoOnce false :!label _label
    (:Completed
      (Audio|SpawnSoundAttached "/Game/Audio/Sounds/Guns/SC_ElectricExplosion_01.SC_ElectricExplosion_01" (Variables|Default|GetRoot))
      (Components|Activation|Activate (Variables|Default|GetSmokeTrail) false)
      (Components|Activation|Deactivate (Variables|Default|GetEngine))
      (Variables|Default|SetPlaneDestroyed true)
      (Variables|Default|Setflying false)
      (Physics|SetSimulatePhysics (Variables|Default|GetFighter) true)
      (Utilities|FlowControl|Delay (Math|Random|RandomFloatinRange 2.0 4.0))
      (Collision|SetCollisionEnabled (Variables|Default|GetFighter) "NoCollision")
      (Components|Activation|Activate (Variables|Default|GetP_Explosion) false)
      (Default|ShipDestroyed (Variables|Default|GetWindRazorGameMode))
      (CallFunction|Reset)
      (goto _label Reset))))

(event Custom|WaveStart
  (CallFunction|Reset)
  (Variables|Default|SetDeactivated false))

(event Custom|EndRaid
  (Variables|Default|SetDeactivated true))

(event Custom|Reset
  (bind _fighter (Variables|Default|GetFighter))
  ;[0.172 1 0] Reset Values
  (Components|Activation|Deactivate (Variables|Default|GetSmokeTrail))
  (Rendering|SetVisibility _fighter false false)
  (Physics|SetSimulatePhysics _fighter false)
  (Variables|Default|SetHealth 2)
  (Variables|Default|Setflying false)
  (Variables|Default|SetdistanceFlown 0.0)
  (if (Variables|Default|GetTestFlight)
    (Utilities|FlowControl|Delay 0.2)
    (else
      (Utilities|FlowControl|Delay (Math|Random|RandomFloatinRange 5.0 1e+01))))
  (Utilities|FlowControl|Sequence
    (:then_0
      (Utilities|FlowControl|DoOnce false) ; enters at Reset
    )
    (:then_1
      (if (not (Variables|Default|GetDeactivated))
        (CallFunction|Respawn)))))

(event Custom|respawn
  (bind _angrysound (Variables|Default|GetAngrySound))
  (bind _engine (Variables|Default|GetEngine))
  ;[0.01863 0.5104 0] Respawn
  (Variables|Default|SetPlaneDestroyed false)
  (if _angrysound
    (Components|Activation|Activate _engine false)
    (else
      (Components|Activation|Activate _engine _angrysound)))
  (Collision|SetCollisionEnabled (Variables|Default|GetFighter) "QueryAndPhysics")
  (Rendering|SetVisibility (Variables|Default|GetFighter) true false)
  (Variables|Default|Setflying true))

(event Custom|Shoot
  ;[1 0.005426 0] Firing Sequence
  (Components|Activation|Activate (Variables|Default|GetRightMuzzleFlash) false)
  (Utilities|FlowControl|Delay (Math|Random|RandomFloatinRange 0.5 1.8))
  (if (Variables|Default|GetPlaneDestroyed)
    (Components|Activation|Deactivate (Variables|Default|GetLeftMuzzleFlash))
    (else
      (Default|DamageShip (Variables|Default|GetWindRazorGameMode) 2)
      (Utilities|FlowControl|Delay (Math|Random|RandomFloatinRange 0.5 1.3))
      (Components|Activation|Deactivate (Variables|Default|GetLeftMuzzleFlash)))))

(event EventBeginPlay
  (bind _aswind_razor_game_mode (Utilities|Casting|CastToWindRazorGameMode (Game|GetGameMode)))
  (Variables|Default|SetWindRazorGameMode _aswind_razor_game_mode)
  (Utilities|FlowControl|Delay (Variables|Default|GetFlightDelay))
  (if (Variables|Default|GetTestFlight)
    (CallFunction|WaveStart)))

(event EventTick
  (params (DeltaSeconds :type Float%20%28single-precision%29))
  (if (Variables|Default|Getflying)
    (bind _output_get (Variables|Default|SetdistanceFlown (+ (Variables|Default|GetdistanceFlown) (* (Variables|Default|GetPlaneBaseSpeed) (Utilities|Time|GetWorldDeltaSeconds) 1e+02))))
    (Transformation|SetWorldTransform (Variables|Default|GetFighter) (Math|Transform|MakeTransform (.location (Spline|GetTransformatDistanceAlongSpline (Variables|Default|GetSpline) _output_get "World" false)) (Math|Rotator|MakeRotator (.roll (.rotation (Spline|GetTransformatDistanceAlongSpline (Variables|Default|GetSpline) _output_get "World" false))) (.pitch (.rotation (Spline|GetTransformatDistanceAlongSpline (Variables|Default|GetSpline) _output_get "World" false))) (.yaw (.rotation (Spline|GetTransformatDistanceAlongSpline (Variables|Default|GetSpline) _output_get "World" false)))) "2.000000,2.000000,2.000000") false false)
    (if (>= (Variables|Default|GetdistanceFlown) (Spline|GetSplineLength (Variables|Default|GetSpline)))
      (if (Variables|Default|GetOneTimeFlight)
        (Variables|Default|SetDeactivated true))
      (CallFunction|Reset)
      (elif (>= (Variables|Default|GetdistanceFlown) (Variables|Default|GetFiring%20Start%20Distance))
        (Utilities|FlowControl|DoOnce false
          (:Completed
            (CallFunction|Shoot)))))))

(event Collision|EventHit
  (params (MyComp :type Primitive%20Component%20Object%20Reference) (Other :type Actor%20Object%20Reference) (OtherComp :type Primitive%20Component%20Object%20Reference) (bSelfMoved :type Boolean) (HitLocation :type Vector :default "0, 0, 0") (HitNormal :type Vector :default "0, 0, 0") (NormalImpulse :type Vector :default "0, 0, 0") (Hit :type Hit%20Result%20Structure%20%28by%20ref%29))
  ;[1 0.1066 0] Damaged on Hit
  (Utilities|Casting|CastToBP_ElectroBullet Other)
  (Effects|SpawnEmitteratLocation "/Game/FX/Eric/P_BulletImpact.P_BulletImpact" HitLocation)
  (if (>= 0 (Variables|Default|GetHealth))
    (CallFunction|DestroyPlane)
    (else
      (Variables|Default|SetHealth (- (Variables|Default|GetHealth) 1)))))

(fn ConstructionScript
  (Transformation|SetWorldLocation (Variables|Default|GetFiringDistanceVisual) (Spline|GetLocationatDistanceAlongSpline (Variables|Default|GetSpline) (Variables|Default|GetFiring%20Start%20Distance) "World") false false))