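; Enemy fighter plane actor that flies a looping route along FlightPath spline points and goes down when hit.
; A latent MoveComponentTo moves the static mesh to the next point, then advances or wraps the index and re-triggers itself through FollowSplineTrail.
; Hit stops movement, fires explosion particles, drops the mesh with physics and removes the actor after a delay.
; Older timeline, spline-distance and AI-controller movement attempts remain disconnected.
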(event Custom|Explode)

(event Custom|FollowSplineTrail
  (Components|MoveComponentTo (Variables|Default|GetStaticMesh) (Spline|GetLocationatSplinePoint (Variables|Default|GetFlightPath) (Variables|Default|GetNextPoint) "World") "0, 0, 0" false false 0.2 false)
  (if (== (Variables|Default|GetNextPoint) (- (Spline|GetNumberOfSplinePoints (Variables|Default|GetFlightPath)) 1))
    (Variables|Default|SetNextPoint 0)
    (CallFunction|FollowSplineTrail)
    (else
      (Variables|Default|SetNextPoint (+ (Variables|Default|GetNextPoint) 1))
      (CallFunction|FollowSplineTrail))))

(event Custom|Destroy
  (Components|MoveComponentTo (Variables|Default|GetStaticMesh) (Spline|GetLocationatSplinePoint (Variables|Default|GetFlightPath) (Variables|Default|GetNextPoint) "World") "0, 0, 0" false false 0.2 false) ; enters at Stop
)

(event EventBeginPlay
  (Components|MoveComponentTo (Variables|Default|GetStaticMesh) (Spline|GetLocationatSplinePoint (Variables|Default|GetFlightPath) (Variables|Default|GetNextPoint) "World") "0, 0, 0" false false 0.2 false)
  (if (== (Variables|Default|GetNextPoint) (- (Spline|GetNumberOfSplinePoints (Variables|Default|GetFlightPath)) 1))
    (Variables|Default|SetNextPoint 0)
    (CallFunction|FollowSplineTrail)
    (else
      (Variables|Default|SetNextPoint (+ (Variables|Default|GetNextPoint) 1))
      (CallFunction|FollowSplineTrail))))

(event EventTick
  (params (DeltaSeconds :type Float%20%28single-precision%29)))

(event Collision|EventHit
  (params (MyComp :type Primitive%20Component%20Object%20Reference) (Other :type Actor%20Object%20Reference) (OtherComp :type Primitive%20Component%20Object%20Reference) (bSelfMoved :type Boolean) (HitLocation :type Vector :default "0, 0, 0") (HitNormal :type Vector :default "0, 0, 0") (NormalImpulse :type Vector :default "0, 0, 0") (Hit :type Hit%20Result%20Structure%20%28by%20ref%29))
  ;[1 1 1] Destroyed on Hit
  (Development|PrintString "BOOM")
  (Components|Activation|Activate (Variables|Default|GetP_Explosion) false)
  (Variables|Default|SetPlaneDestroyed true)
  (CallFunction|Destroy)
  (Physics|SetEnableGravity (Variables|Default|GetStaticMesh) true)
  (Physics|SetSimulatePhysics (Variables|Default|GetStaticMesh) true)
  (Utilities|FlowControl|Delay 1e+01)
  (Actor|DestroyActor))

(fn ConstructionScript)