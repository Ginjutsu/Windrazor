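; BP_SwayingPlane is a blockout actor that sways its static mesh back and forth around its starting world location.
; On BeginPlay it waits a random delay to desynchronize instances, caches that location, then runs the PlaneLoc timeline, adding its vector offset each update.
; When the timeline finishes, a short pause and the PlayedOnce flag alternate reverse and forward playback, producing an endless ping-pong.
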(event EventBeginPlay
  (Utilities|FlowControl|Delay (Math|Random|RandomFloatinRange 0.0 1e+01))
  (Variables|Default|SetInitLoc (Transformation|GetWorldLocation (Variables|Default|GetStaticMesh)))
  (bind _planeloc (Timeline|PlaneLoc Play)
    (:Update
      (Transformation|SetWorldLocation (Variables|Default|GetStaticMesh) (+ _planeloc (Variables|Default|GetInitLoc)) false false))
    (:Finished
      (Utilities|FlowControl|Delay 0.2)
      (if (Variables|Default|GetPlayedOnce)
        (Variables|Default|SetPlayedOnce false)
        (Timeline|PlaneLoc PlayFromStart)
        (else
          (Variables|Default|SetPlayedOnce true)
          (Timeline|PlaneLoc Reverse))))))

(fn ConstructionScript)